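; Player controller for a session-based multiplayer game that drives the main game HUD, player list, chat and kick handling.
; It creates the MainGame widget and forwards player count and list updates, while P and Enter open the list and chat box with matching input modes.
; Chat messages fan out through the GameMode's controller list to each chat window and into chat history.
; Kicks open a Kicked or ServerFull level and destroy the session.
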(event `Key|P`
  (params (Key :type "Key Structure"))
  (bind _maingame_wb (`self.MainGame_WB`))
  ;[1 1 1] Controls
  ;;[1 1 1] Showing and hiding player list in main game WB
  (:`Pressed`
    (if (`self.PlayerListVisible?`)
      (`/Game/UI/MainGame_WB.Hide Player List` _maingame_wb)
      (set `self.PlayerListVisible?` false)
      (`WidgetBlueprintLibrary.SetInputMode_GameOnly` self)
      (set `self.bShowMouseCursor` false)
      (else
        (`/Game/UI/MainGame_WB.Show Player List` _maingame_wb)
        (set `self.PlayerListVisible?` true)
        (`WidgetBlueprintLibrary.SetInputMode_GameAndUIEx` self null "DoNotLock" false)
        (set `self.bShowMouseCursor` true)))))

(event `Update Number Of Players`
  (params (CurrentPlayers :type Integer))
  (set `/Game/UI/MainGame_WB.CurrentPlayers` CurrentPlayers (`self.MainGame_WB`)))

(event `Add Main Game WB`
  (params (ServerSlots :type Integer))
  ;[1 1 1] Function to add main game widget
  (bind _returnvalue (`|CreateWidget` "/Game/UI/MainGame_WB.MainGame_WB_C" self ServerSlots))
  (bind _output_get (set `self.MainGame_WB` _returnvalue))
  (`UserWidget.AddToViewport` _output_get 0))

(event `Key|Enter`
  (params (Key :type "Key Structure"))
  ;[1 1 1] Controls
  ;;[1 1 1] Showing and hiding chat type box in main game WB
  (:`Pressed`
    (`/Game/UI/ChatWindow_WB.Show Type Box` (`/Game/UI/MainGame_WB.ChatWindow_WB` (`self.MainGame_WB`)))
    (`WidgetBlueprintLibrary.SetInputMode_GameAndUIEx` self (`/Game/UI/ChatWindow_WB.Message_TextBox` (`/Game/UI/MainGame_WB.ChatWindow_WB` (`self.MainGame_WB`))) "DoNotLock" false)
    (set `self.bShowMouseCursor` true)))

(event `Add Player To List`
  (params (Player :type Text) (PlayerIndex :type Integer))
  (`/Game/UI/MainGame_WB.Add Player To List` (`self.MainGame_WB`) Player PlayerIndex))

(event `Clear Player List`
  (`/Game/UI/MainGame_WB.Clear Player List` (`self.MainGame_WB`)))

(event `Kick`
  (params (KickIndex :type Integer))
  ;[1 1 1] Function for kick
  (switch `int` KickIndex
    (:`Default`
      (`GameplayStatics.OpenLevel` "Kicked" :!label _label)
      (`DestroySessionCallbackProxy.DestroySession` self))
    (:`0`
      (goto _label))
    (:`1`
      (`GameplayStatics.OpenLevel` "ServerFull")
      (`DestroySessionCallbackProxy.DestroySession` self))))

(event `Add Message From Server To Earch Player`
  (params (Message :type String) (Color :type "SlateColor Structure") (`isServerMessage?` :type Boolean))
  (bind _chatmessagestructure (make `/Game/Blueprints/ChatMessageStructure` (`AdvancedSessionsLibrary.GetPlayerName` self) Message Color `isServerMessage?`))
  (bind _asmain_game_mode (cast `/Game/Blueprints/MainGameMode` (`GameplayStatics.GetGameMode`)))
  (for _array_element (`/Game/Blueprints/MainGameMode.AllPCs` _asmain_game_mode)
    (bind _asmain_player_controller (cast `/Game/Blueprints/MainPlayerController` _array_element))
    (`self.Add Message To Chat` _asmain_player_controller _chatmessagestructure))
  (bind _asmain_game_mode_2 (cast `/Game/Blueprints/MainGameMode` (`GameplayStatics.GetGameMode`)))
  (`/Game/Blueprints/MainGameMode.Add Message To Chat History` _asmain_game_mode_2 _chatmessagestructure))

(event `Add Message To Chat`
  (params (ChatData :type "/Game/Blueprints/ChatMessageStructure Structure"))
  (`/Game/UI/ChatWindow_WB.Add Child To Chat` (`/Game/UI/MainGame_WB.ChatWindow_WB` (`self.MainGame_WB`)) ChatData))

(fn `UserConstructionScript`)