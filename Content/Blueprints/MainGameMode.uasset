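; Game mode for a multiplayer session that tracks connected players, enforces the slot limit and relays join and leave messages to chat.
; On login the authority stores the controller, reads slots from the game instance, builds the main widget and replays the logged chat history to the newcomer.
; UpdateServer kicks the newest player when over capacity, then rebuilds every client's player list and count.
; Logout announces the departure and refreshes everyone.
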(event `Send Server Message`
  (params (Message :type String))
  ;[1 1 1] Send server message
  (bind _asmain_player_controller (cast `/Game/Blueprints/MainPlayerController` (`GameplayStatics.GetPlayerController` 0)))
  (`/Game/Blueprints/MainPlayerController.Add Message From Server To Earch Player` _asmain_player_controller Message (make `SlateColor` (struct :`R` 1.0 :`A` 1.0)) true))

(event `Add Message To Chat History`
  (params (`Message Data` :type "/Game/Blueprints/ChatMessageStructure Structure"))
  ;[1 1 1] Load message history
  (`KismetArrayLibrary.Array_Add` (`self.MessageLog`) `Message Data`))

(event `self.K2_PostLogin`
  (params (NewPlayer :type "PlayerController Object Reference"))
  ;[1 1 1] Adding player to player list
  (`self.Send Server Message` (`KismetStringLibrary.Concat_StrStr` (`AdvancedSessionsLibrary.GetPlayerName` NewPlayer) " joined."))
  (`/Engine/EditorBlueprintResources/ActorMacros.Switch Has Authority`
    (:`Authority`
      (`KismetArrayLibrary.Array_Add` (`self.AllPCs`) NewPlayer)
      (bind _asmy_game_instance (cast `/Game/Blueprints/MyGameInstance` (`GameplayStatics.GetGameInstance`)))
      (set `self.ServerSlots` (`/Game/Blueprints/MyGameInstance.ServerSlots` _asmy_game_instance))
      (bind _asmain_player_controller (cast `/Game/Blueprints/MainPlayerController` NewPlayer))
      (`/Game/Blueprints/MainPlayerController.Add Main Game WB` _asmain_player_controller (`self.ServerSlots`))
      (`self.Update Server`)
      ;[1 1 1] Load message history
      (for _array_element (`self.MessageLog`)
        (bind _asmain_player_controller_2 (cast `/Game/Blueprints/MainPlayerController` NewPlayer))
        (`/Game/Blueprints/MainPlayerController.Add Message To Chat` _asmain_player_controller_2 _array_element)))))

(event `Update Server`
  (bind _returnvalue (`KismetArrayLibrary.Array_Length` (`self.AllPCs`)))
  ;[1 1 1] Updating player list and whole server
  (if (> _returnvalue (`self.ServerSlots`))
    (`self.Kick Player` (- _returnvalue 1) 1)
    (`KismetSystemLibrary.Delay` 0.2))
  (for _array_element (`self.AllPCs`)
    (bind _asmain_player_controller (cast `/Game/Blueprints/MainPlayerController` _array_element))
    (`/Game/Blueprints/MainPlayerController.Clear Player List` _asmain_player_controller)
    (for (_array_element_2 _array_index) (`self.AllPCs`)
      (`/Game/Blueprints/MainPlayerController.Add Player To List` _asmain_player_controller (`KismetTextLibrary.Conv_StringToText` (`AdvancedSessionsLibrary.GetPlayerName` _array_element_2)) _array_index)))
  (for _array_element_3 (`self.AllPCs`)
    (bind _asmain_player_controller_2 (cast `/Game/Blueprints/MainPlayerController` _array_element_3))
    (`/Game/Blueprints/MainPlayerController.Update Number Of Players` _asmain_player_controller_2 (`KismetArrayLibrary.Array_Length` (`self.AllPCs`)))))

(event `Kick Player`
  (params (Index :type Integer) (KickIndex :type Integer))
  ;[1 1 1] Kick ?
  (bind _asmain_player_controller (cast `/Game/Blueprints/MainPlayerController` (`|GetArrayItem` (`self.AllPCs`) Index)))
  (`/Game/Blueprints/MainPlayerController.Kick` _asmain_player_controller KickIndex))

(event `self.K2_OnLogout`
  (params (ExitingController :type "Controller Object Reference"))
  (bind _allpcs (`self.AllPCs`))
  ;[1 1 1] Remove someone from player list when they leave
  (for (_array_element _array_index) _allpcs
    (if (== ExitingController _array_element)
      (`self.Send Server Message` (`KismetStringLibrary.Concat_StrStr` (`AdvancedSessionsLibrary.GetPlayerName` _array_element) " left."))
      (break)))
  (`KismetArrayLibrary.Array_Remove` _allpcs _array_index)
  (`self.Update Server`))

(fn `UserConstructionScript`)