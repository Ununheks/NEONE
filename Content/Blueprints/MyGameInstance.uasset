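; Game instance that creates a multiplayer lobby session and hosts its map.
; The CreateLobby event stores the server settings, then creates an advanced session with name, map, LAN flag and password data as extra properties.
; Public connections are the requested slots plus a fixed offset of three, and the LAN flag also sets the session's LAN mode.
; On success it opens the chosen map as a listen server.
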(event `CreateLobby`
  (params (ServerName :type String) (ServerMap :type String) (ServerSlots :type Integer) (`ServerMethod_Lan?` :type Boolean) (Password :type String) (`HasPassword?` :type Boolean))
  (set `self.ServerName` ServerName)
  (set `self.ServerMap` ServerMap)
  (set `self.ServerSlots` ServerSlots)
  (set `self.ServerMethod_Lan?` `ServerMethod_Lan?`)
  (set `self.Password` Password)
  (set `self.HasPassword?` `HasPassword?`)
  (`CreateSessionCallbackProxyAdvanced.CreateAdvancedSession` (`|MakeArray` (`AdvancedSessionsLibrary.MakeLiteralSessionPropertyString` "NAME" (`self.ServerName`)) (`AdvancedSessionsLibrary.MakeLiteralSessionPropertyString` "MAP" (`self.ServerMap`)) (`AdvancedSessionsLibrary.MakeLiteralSessionPropertyBool` "LAN" (`self.ServerMethod_Lan?`)) (`AdvancedSessionsLibrary.MakeLiteralSessionPropertyString` "PASSWORD" (`self.Password`)) (`AdvancedSessionsLibrary.MakeLiteralSessionPropertyBool` "HASPASSWORD" (`self.HasPassword?`))) (`GameplayStatics.GetPlayerController` 0) (+ (`self.ServerSlots`) 3) 0 (`self.ServerMethod_Lan?`)
    (:`OnSuccess`
      (`GameplayStatics.OpenLevel` (`KismetStringLibrary.Conv_StringToName` (`self.ServerMap`)) true "listen"))))